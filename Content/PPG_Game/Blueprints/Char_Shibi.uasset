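; Shibi character Blueprint that manages Health and Mana attributes and shows them as glass-ball gauges on the main HUD widget.
; BeginPlay creates the HUD and stores each ball widget in its struct within an enum-keyed Attributes map.
; ModifyAttribute clamps changes, then UpdateAttribute drives the ball's dynamic material fill, with Health also HSV-lerping from red to its widget color.
; Subtract and Add keys lower or raise Health.
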(event `self.ReceiveBeginPlay`
  (bind _returnvalue (`|CreateWidget` "/Game/PPG_Game/UI/W_PC_Main.W_PC_Main_C"))
  (bind _output_get (set `self.MasterWidget` _returnvalue))
  (`self.SetupAttributeBars`)
  (`self.UpdateAttribute` "NewEnumerator0")
  (`self.UpdateAttribute` "NewEnumerator1")
  (`UserWidget.AddToViewport` _output_get 0))

(event `Key|Subtract`
  (params (Key :type "Key Structure"))
  (:`Pressed`
    (`self.ModifyAttribute` "NewEnumerator0" -30.0)))

(event `Key|Add`
  (params (Key :type "Key Structure"))
  (:`Pressed`
    (`self.ModifyAttribute` "NewEnumerator0" 30.0)))

(fn `GetAttribute`
  (params (Attribute :type "/Game/PPG_Game/Blueprints/Enum/E_Attribute Enum" :default "NewEnumerator0"))
  (returns (Value :type "/Game/PPG_Game/Blueprints/Structure/S_Attribute Structure"))
  (return (`BlueprintMapLibrary.Map_Find` (`self.Attributes`) Attribute)))

(fn `ModifyAttribute`
  (params (Attribute :type "/Game/PPG_Game/Blueprints/Enum/E_Attribute Enum" :default "NewEnumerator3") (ModifyValue :type "Float (double-precision)"))
  (locals (LocalAttribute :type "/Game/PPG_Game/Blueprints/Enum/E_Attribute Enum" :default "NewEnumerator3") (LocalModifyValue :type "Float (double-precision)"))
  (bind _localattribute (`local.LocalAttribute`))
  (bind _value (`self.GetAttribute` (`local.LocalAttribute`)))
  (bind (_currentvalue _minvalue _maxvalue) (break `/Game/PPG_Game/Blueprints/Structure/S_Attribute` _value))
  (set `local.LocalAttribute` Attribute)
  (set `local.LocalModifyValue` ModifyValue)
  (bind _structout (setmembers `/Game/PPG_Game/Blueprints/Structure/S_Attribute` :`StructRef` _value :`CurrentValue` (`KismetMathLibrary.FClamp` (+ _currentvalue (`local.LocalModifyValue`)) _minvalue _maxvalue)))
  (`self.SetAttribute` _structout _localattribute)
  (`self.UpdateAttribute` _localattribute)
  (return))

(fn `SetAttribute`
  (params (Value :type "/Game/PPG_Game/Blueprints/Structure/S_Attribute Structure (by ref)") (Attribute :type "/Game/PPG_Game/Blueprints/Enum/E_Attribute Enum" :default "NewEnumerator0"))
  (`BlueprintMapLibrary.Map_Add` (`self.Attributes`) Attribute Value)
  (return))

(fn `SetupAttributeBars`
  (bind _masterwidget (`self.MasterWidget`))
  (bind _structout (setmembers `/Game/PPG_Game/Blueprints/Structure/S_Attribute` :`StructRef` (`self.GetAttribute` "NewEnumerator0") :`GlassBallWidget` (`/Game/PPG_Game/UI/W_PC_Main.Health` _masterwidget)))
  (`self.SetAttribute` _structout "NewEnumerator0")
  (bind _structout_2 (setmembers `/Game/PPG_Game/Blueprints/Structure/S_Attribute` :`StructRef` (`self.GetAttribute` "NewEnumerator1") :`GlassBallWidget` (`/Game/PPG_Game/UI/W_PC_Main.Mana` _masterwidget)))
  (`self.SetAttribute` _structout_2 "NewEnumerator1"))

(fn `UpdateAttribute`
  (params (Attribute :type "/Game/PPG_Game/Blueprints/Enum/E_Attribute Enum" :default "NewEnumerator0"))
  (returns (Value :type "/Game/PPG_Game/Blueprints/Structure/S_Attribute Structure"))
  (bind (_currentvalue _minvalue _maxvalue _glassballwidget) (break `/Game/PPG_Game/Blueprints/Structure/S_Attribute` (`self.GetAttribute` Attribute)))
  (bind _returnvalue (`KismetMathLibrary.FClamp` (/ _currentvalue _maxvalue)))
  (`/Engine/EditorBlueprintResources/StandardMacros.IsValid` _glassballwidget
    (:`Is Valid`
      (bind _returnvalue_2 (`Image.GetDynamicMaterial` (`/Game/PPG_Game/UI/W_GlassBall.GlassBall` _glassballwidget)))
      (`MaterialInstanceDynamic.SetScalarParameterValue` _returnvalue_2 "Percentage" _returnvalue)
      (if (`|EnumEquality` Attribute "NewEnumerator0")
        (`MaterialInstanceDynamic.SetVectorParameterValue` _returnvalue_2 "Color" (`KismetMathLibrary.LinearColorLerpUsingHSV` (struct :`R` 1.0 :`A` 1.0) (`/Game/PPG_Game/UI/W_GlassBall.Color` _glassballwidget) _returnvalue))
        (return)))
    (:`Is Not Valid`
      (return))))

(fn `UserConstructionScript`
  (`parent.UserConstructionScript`))