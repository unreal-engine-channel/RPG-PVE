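; BP_RPG_NPC is a quest-giver NPC that shows its name widget while the player (Char_Shibi) is inside its sphere.
; Player level updates step through a level-to-quest map, unlocking the next quest and switching the sprite to a question mark.
; Interacting in range adds that quest to the player's QuestManage and reverts the sprite to a circle.
; The player is set as owner so the marker sprite is hidden from their own view.
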(event `self.ReceiveBeginPlay`
  (bind _shibi (`self.Shibi`))
  (bind _aschar_shibi (cast `/Game/PPG_Game/Blueprints/Char_Shibi` (`GameplayStatics.GetPlayerCharacter` 0)))
  (set `self.Shibi` _aschar_shibi)
  (`self.SetOwner` _aschar_shibi)
  (`PrimitiveComponent.SetOwnerNoSee` (`self.PaperSprite`) true)
  (bind _asw_name_for_npc (cast `/Game/PPG_Game/UI/W_NameForNPC` (`WidgetComponent.GetUserWidgetObject` (`self.Widget`))))
  (`TextBlock.SetText` (`/Game/PPG_Game/UI/W_NameForNPC.Name` _asw_name_for_npc) (`self.Name`))
  (add `/Game/PPG_Game/Blueprints/Char_Shibi.OnInteract` _shibi (`|CreateDelegate` :!event `OnInteract`))
  (add `/Game/PPG_Game/Blueprints/Char_Shibi.UpdateLevelForQuest` _shibi (`|CreateDelegate` :!event `UpdateQuest`))
  (`self.UpdateQuest` 0))

(event `OnInteract`
  (if (and (`self.HasQuest?`) (`self.InRadius?`) (`KismetSystemLibrary.IsValidClass` (`self.CurrentQuestClass`)))
    (`/Game/PPG_Game/Component/QuestManager.AddQuest` (`/Game/PPG_Game/Blueprints/BP_RPG_Character.QuestManage` (`self.Shibi`)) (`self.CurrentQuestClass`))
    (set `self.HasQuest?` false)
    (`PaperSpriteComponent.SetSprite` (`self.PaperSprite`) "/Game/PPG_Game/Textures/circle_Sprite.circle_Sprite")))

(event `self.Sphere.OnComponentBeginOverlap`
  (params (OverlappedComponent :type "PrimitiveComponent Object Reference") (OtherActor :type "Actor Object Reference") (OtherComp :type "PrimitiveComponent Object Reference") (OtherBodyIndex :type Integer) (bFromSweep :type Boolean) (SweepResult :type "HitResult Structure (by ref)"))
  (if (== OtherActor (`self.Shibi`))
    (`SceneComponent.SetHiddenInGame` (`self.Widget`) false false)
    (set `self.InRadius?` true)))

(event `self.Sphere.OnComponentEndOverlap`
  (params (OverlappedComponent :type "PrimitiveComponent Object Reference") (OtherActor :type "Actor Object Reference") (OtherComp :type "PrimitiveComponent Object Reference") (OtherBodyIndex :type Integer))
  (if (== OtherActor (`self.Shibi`))
    (`SceneComponent.SetHiddenInGame` (`self.Widget`) true false)
    (set `self.InRadius?` false)))

(event `UpdateQuest`
  (params (Level :type Integer))
  (bind _questinlevel (`self.QuestInLevel`))
  (bind _keys (`BlueprintMapLibrary.Map_Keys` _questinlevel))
  (bind _output (`|GetArrayItem` _keys (`self.LevelIndex`)))
  (bind _value (`BlueprintMapLibrary.Map_Find` _questinlevel _output))
  (if (and (>= Level _output) (`KismetSystemLibrary.IsValidClass` _value) (!= (`self.CurrentQuestClass`) _value))
    (set `self.HasQuest?` true)
    (`PaperSpriteComponent.SetSprite` (`self.PaperSprite`) "/Game/PPG_Game/Textures/question_mark_Sprite.question_mark_Sprite")
    (set `self.CurrentQuestClass` _value)
    (`/Engine/EditorBlueprintResources/StandardMacros.IncrementInt` (`self.LevelIndex`))))

(fn `UserConstructionScript`
  (`parent.UserConstructionScript`))