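; BP_MasterQuest is a quest actor, apparently a base class, that tracks which sub-goals are currently active.
; SetupStartingSubGoals activates the starting indices, and UpdateSubGoalsInfo rebuilds the current sub-goal data from QuestInfo using those indices.
; GoToNextSubGoal replaces all active sub-goals with the one after the highest current index, returning false when none remains.
; The event graph and construction script are empty.
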(fn `GoToNextSubGoal`
  (returns (Success :type Boolean))
  (locals (LocalNextIndex :type Integer :default 0))
  (bind _currentsubgoalindices (`self.CurrentSubGoalIndices`))
  (bind _returnvalue (+ (`.MaxValue` (`KismetMathLibrary.MaxOfIntArray` (`self.CurrentSubGoalIndices`))) 1))
  (if (<= _returnvalue (`KismetArrayLibrary.Array_LastIndex` (`.SubGoalInfo_18_1962D1FF4A2E9B808EBF31A288F58A89` (break `/Game/PPG_Game/Blueprints/Structure/S_QuestInfo` (`self.QuestInfo`)))))
    (set `local.LocalNextIndex` _returnvalue)
    (`KismetArrayLibrary.Array_Clear` _currentsubgoalindices)
    (`KismetArrayLibrary.Array_Add` _currentsubgoalindices (`local.LocalNextIndex`))
    (`self.UpdateSubGoalsInfo`)
    (return true)
    (else
      (return false))))

(fn `SetupStartingSubGoals`
  (`KismetArrayLibrary.Array_Clear` (`self.CurrentSubGoalIndices`))
  (set `self.CurrentSubGoalIndices` (`self.StartSubGoalIndices`))
  (`self.UpdateSubGoalsInfo`))

(fn `UpdateSubGoalsInfo`
  (`KismetArrayLibrary.Array_Clear` (`self.CurrentSubGoalInfo`))
  (for _array_element (`self.CurrentSubGoalIndices`)
    (`KismetArrayLibrary.Array_Add` (`self.CurrentSubGoalInfo`) (`|GetArrayItem` (`.SubGoalInfo_18_1962D1FF4A2E9B808EBF31A288F58A89` (break `/Game/PPG_Game/Blueprints/Structure/S_QuestInfo` (`self.QuestInfo`))) _array_element))))

(fn `UserConstructionScript`)