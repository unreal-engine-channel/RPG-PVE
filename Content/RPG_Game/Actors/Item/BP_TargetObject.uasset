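; BP_TargetObject is an interactable world object that shows a floating interaction prompt through a widget component.
; On BeginPlay it fills the W_Interaction widget with its Name and Interact text and tints the name blue.
; Begin and end overlap events toggle the widget's visibility.
; OnInteractwith is an empty stub, so the object itself defines no interaction behavior.
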(event `self.ReceiveBeginPlay`
  (bind _asw_interaction (cast `/Game/RPG_Game/UI/W_Interaction` (`WidgetComponent.GetUserWidgetObject` (`self.Widget`)) :!pure true))
  (bind _name (`/Game/RPG_Game/UI/W_Interaction.Name` _asw_interaction))
  (`TextBlock.SetText` _name (`self.Name`))
  (`TextBlock.SetColorAndOpacity` _name (make `SlateColor` (struct :`R` 0.180818 :`G` 0.269838 :`B` 1.0 :`A` 1.0)))
  (`TextBlock.SetText` (`/Game/RPG_Game/UI/W_Interaction.Interact` _asw_interaction) (`self.Interact`)))

(event `/Game/RPG_Game/Blueprints/Interface/I_Interaction.BeginOverlapTargetObject`
  (`SceneComponent.SetVisibility` (`self.Widget`) true false))

(event `/Game/RPG_Game/Blueprints/Interface/I_Interaction.EndOverlapTargetObject`
  (`SceneComponent.SetVisibility` (`self.Widget`) false false))

(event `/Game/RPG_Game/Blueprints/Interface/I_Interaction.OnInteractWith`
  (params (Character :type "/Game/RPG_Game/Blueprints/BP_Player Object Reference")))

(fn `UserConstructionScript`)