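; BP_MasterQuest holds one quest's runtime state: active and completed sub-goals, hunt counters and a growing description.
; CompleteSubGoal retires a goal's widget, records success or failure, and refreshes the mission menu when this quest is selected.
; When no active goals remain, UpdateCompletedSubGoal branches to following indices, polling with a short Delay until old widgets clear, or plays the quest widget out.
; GoToNextSubGoal offers linear advancement by index.
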(event `UpdateCompletedSubGoal`
  (bind _currentsubgoalinfo (`self.CurrentSubGoalInfo`))
  (bind _manager_w_quest (`self.Manager_W_Quest`))
  (bind _output (`|GetArrayItem` (`/Game/RPG_Game/UI/W_Quest.SubGoalWidgets` _manager_w_quest)))
  (for _array_element (`self.CompletedSubGoalsInfo`)
    (bind (_subgoalindex _subgoalinfo) (break `/Game/RPG_Game/Blueprints/Structure/S_CompletedSubGoalInfo` _array_element))
    (bind (_type _customsubgoal_ _customsubgoaltext _targetname _amounttohunt _targetlocation _canupdatequestdescription_ _updatedescription _followingsubgoalindices _targetclass _targetclassid _hasfollowingindex_) (break `/Game/RPG_Game/Blueprints/Structure/S_SubGoalInfo` _subgoalinfo))
    (set `self.IsFinished?` _hasfollowingindex_)
    (if _hasfollowingindex_
      (`KismetArrayLibrary.Array_Clear` _currentsubgoalinfo)
      (setmembers `/Game/RPG_Game/Blueprints/Structure/S_SubGoalInfo` :`StructRef` _subgoalinfo)
      (for _array_element_2 _followingsubgoalindices
        (bind _returnvalue (`KismetArrayLibrary.Array_Add` (`self.CurrentSubGoalIndices`) _array_element_2))
        (`KismetArrayLibrary.Array_Add` (`self.CurrentHuntedAmount`))
        (`KismetArrayLibrary.Array_Add` _currentsubgoalinfo))
      (break)))
  (if (`self.IsFinished?`)
    (`/Game/RPG_Game/UI/W_Quest.PlaySubGoal` _manager_w_quest false)
    (if (not (`KismetSystemLibrary.IsValid` _output)) :!label _label
      (`/Game/RPG_Game/UI/W_Quest.GenerateSubGoal` _manager_w_quest)
      (`/Game/RPG_Game/UI/W_Quest.SelectSubGoal` _manager_w_quest _output)
      (`/Game/RPG_Game/UI/W_Quest.PlaySubGoal` _manager_w_quest true)
      (else
        (`KismetSystemLibrary.Delay` 0.01)
        (goto _label)))
    (else
      (`/Game/RPG_Game/UI/W_Quest.PlayQuest` _manager_w_quest false))))

(fn `CompleteSubGoal`
  (params (SubGoalIndex :type Integer) (`Success?` :type Boolean))
  (locals (LocalCompletedSubGoalIndex :type Integer) (LocalCompletedSubGoalInfo :type "/Game/RPG_Game/Blueprints/Structure/S_SubGoalInfo Structure") (LocalSuccess :type Boolean))
  (bind _manager_w_quest (`self.Manager_W_Quest`))
  (bind _currentsubgoalindices (`self.CurrentSubGoalIndices`))
  (bind _localcompletedsubgoalindex (`local.LocalCompletedSubGoalIndex`))
  (bind _returnvalue (`KismetArrayLibrary.Array_Find` _currentsubgoalindices _localcompletedsubgoalindex))
  (bind _subgoalwidgets (`/Game/RPG_Game/UI/W_Quest.SubGoalWidgets` (`self.Manager_W_Quest`)))
  (bind _output (`|GetArrayItem` (`.SubGoalInfo_18_1962D1FF4A2E9B808EBF31A288F58A89` (break `/Game/RPG_Game/Blueprints/Structure/S_QuestInfo` (`self.QuestInfo`))) (`local.LocalCompletedSubGoalIndex`)))
  (bind _output_2 (`|GetArrayItem` _subgoalwidgets (`KismetArrayLibrary.Array_Find` (`self.CurrentSubGoalIndices`) (`local.LocalCompletedSubGoalIndex`))))
  (bind ((`CanUpdateQuestDescription?_19_54F443454EC5709BD12A59BFA4630268` _canupdatequestdescription_) (`UpdateDescription_22_1944844E473FF43C354D37B6DDC1F0D1` _updatedescription)) (break `/Game/RPG_Game/Blueprints/Structure/S_SubGoalInfo` _output))
  (set `local.LocalCompletedSubGoalIndex` SubGoalIndex)
  (set `local.LocalSuccess` `Success?`)
  (if (`KismetArrayLibrary.Array_Contains` (`self.CurrentSubGoalIndices`) (`local.LocalCompletedSubGoalIndex`))
    (`/Game/RPG_Game/UI/W_SubGoal.DisableButton` _output_2 (`local.LocalSuccess`))
    (`KismetArrayLibrary.Array_RemoveItem` _subgoalwidgets _output_2)
    (`KismetArrayLibrary.Array_Remove` (`self.CurrentHuntedAmount`) _returnvalue)
    (`KismetArrayLibrary.Array_RemoveItem` _currentsubgoalindices _returnvalue)
    (bind _output_get (set `local.LocalCompletedSubGoalInfo` _output))
    (if _canupdatequestdescription_
      (set `self.CurrentDescripiton` (`|FormatText` "{Current} {New}" (`self.CurrentDescripiton`) _updatedescription))
      (if (`self.SelectInMission`)
        (`/Game/RPG_Game/UI/W_Mission.UpdateDescription` (`/Game/RPG_Game/UI/W_PC_Main.W_Mission` (`self.Manager_PC_Main`)))
        (`KismetArrayLibrary.Array_Add` (`self.CompletedSubGoalsInfo`) (make `/Game/RPG_Game/Blueprints/Structure/S_CompletedSubGoalInfo` _localcompletedsubgoalindex _output_get (`local.LocalSuccess`)) :!label _label)
        (`KismetArrayLibrary.Array_RemoveItem` (`self.CurrentSubGoalInfo`) (`local.LocalCompletedSubGoalInfo`))
        (if (not (`KismetArrayLibrary.Array_IsValidIndex` (`self.CurrentSubGoalIndices`)))
          (`self.UpdateCompletedSubGoal`)
          (else
            (if (`self.SelectInMission`)
              (`/Game/RPG_Game/UI/W_Mission.GenerateSubGoals` (`/Game/RPG_Game/UI/W_PC_Main.W_Mission` (`self.Manager_PC_Main`))))
            (if (and (== (`local.LocalCompletedSubGoalIndex`) (`self.SelectedSubGoalIndex`)) (== (`/Game/RPG_Game/Component/QuestManager.CurrentQuest` (`self.QuestManager`)) self))
              (`/Game/RPG_Game/UI/W_Quest.SelectSubGoal` _manager_w_quest (`|GetArrayItem` (`/Game/RPG_Game/UI/W_Quest.SubGoalWidgets` _manager_w_quest) (`|GetArrayItem` (`self.CurrentSubGoalIndices`))))))))
      (else
        (goto _label)))))

(fn `GoToNextSubGoal`
  (returns (Success :type Boolean))
  (locals (LocalNextIndex :type Integer :default 0))
  (bind _currentsubgoalindices (`self.CurrentSubGoalIndices`))
  (bind _returnvalue (+ (`.MaxValue` (`KismetMathLibrary.MaxOfIntArray` (`self.CurrentSubGoalIndices`))) 1))
  (if (<= _returnvalue (`KismetArrayLibrary.Array_LastIndex` (`.SubGoalInfo_18_1962D1FF4A2E9B808EBF31A288F58A89` (break `/Game/RPG_Game/Blueprints/Structure/S_QuestInfo` (`self.QuestInfo`)))))
    (set `local.LocalNextIndex` _returnvalue)
    (`KismetArrayLibrary.Array_Clear` _currentsubgoalindices)
    (`KismetArrayLibrary.Array_Add` _currentsubgoalindices (`local.LocalNextIndex`))
    (`self.UpdateSubGoalsInfo`)
    (return true)
    (else
      (return false))))

(fn `SelectInMission`
  (returns (ReturnValue :type Boolean))
  (bind _selectedquest (`/Game/RPG_Game/UI/W_Mission.SelectedQuest` (`/Game/RPG_Game/UI/W_PC_Main.W_Mission` (`self.Manager_PC_Main`))))
  (return (and (== (`/Game/RPG_Game/Component/QuestManager.CurrentQuest` (`self.QuestManager`)) _selectedquest) (`KismetSystemLibrary.IsValid` _selectedquest))))

(fn `SetupStartingSubGoals`
  (bind _startsubgoalindices (`self.StartSubGoalIndices`))
  (`KismetArrayLibrary.Array_Clear` (`self.CurrentSubGoalIndices`))
  (set `self.CurrentSubGoalIndices` _startsubgoalindices)
  (`KismetArrayLibrary.Array_Resize` (`self.CurrentHuntedAmount`) (`KismetArrayLibrary.Array_Length` _startsubgoalindices))
  (`self.UpdateSubGoalsInfo`)
  (set `self.CurrentDescripiton` (`.Descripion_8_522F3A2141FE9CBA2D954EB228C5F8F1` (break `/Game/RPG_Game/Blueprints/Structure/S_QuestInfo` (`self.QuestInfo`)))))

(fn `UpdateSubGoalsInfo`
  (`KismetArrayLibrary.Array_Clear` (`self.CurrentSubGoalInfo`))
  (for _array_element (`self.CurrentSubGoalIndices`)
    (`KismetArrayLibrary.Array_Add` (`self.CurrentSubGoalInfo`) (`|GetArrayItem` (`.SubGoalInfo_18_1962D1FF4A2E9B808EBF31A288F58A89` (break `/Game/RPG_Game/Blueprints/Structure/S_QuestInfo` (`self.QuestInfo`))) _array_element))))

(fn `UserConstructionScript`)