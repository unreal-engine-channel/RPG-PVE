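; BP_XP is an experience pickup actor that flies to the player and grants XP.
; On BeginPlay it waits a short random delay, turns off physics on its sphere and records its location.
; A MoveToPlayer timeline then lerps it from there to the player's current position each update.
; When the timeline finishes, it destroys itself and adds its XPPoints to the player.
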(event `self.ReceiveBeginPlay`
  (`KismetSystemLibrary.Delay` (`KismetMathLibrary.RandomFloatInRange` 0.5 1.5))
  (`PrimitiveComponent.SetSimulatePhysics` (`self.Sphere`) false)
  (set `self.InitActorLocation` (`self.K2_GetActorLocation`))
  (bind (_direction _alpha) (`Timeline|MoveToPlayer`)
    (:`Update`
      (`self.K2_SetActorLocation` (`KismetMathLibrary.VLerp` (`self.InitActorLocation`) (`self.K2_GetActorLocation` (`self.Player`)) _alpha)))
    (:`Finished`
      (`self.FinishCollect`))))

(event `FinishCollect`
  (`self.K2_DestroyActor`)
  (`/Game/RPG_Game/Blueprints/BP_Player.AddXP` (`self.Player`) (`self.XP_Points`)))

(fn `UserConstructionScript`)