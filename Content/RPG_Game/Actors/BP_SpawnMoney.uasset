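; BP_SpawnMoney is a money pickup actor that flies to the player and collects itself, with no overlap needed.
; After a short random delay on BeginPlay, it disables physics on its Sphere and records its location.
; The MoveToPlayer timeline lerps it toward the Player's live position.
; On finish, it adds Money through the RPG_PlayerController's inventory manager and destroys itself.
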(event `self.ReceiveBeginPlay`
  (`KismetSystemLibrary.Delay` (`KismetMathLibrary.RandomFloatInRange` 0.5 1.5))
  (`PrimitiveComponent.SetSimulatePhysics` (`self.Sphere`) false)
  (set `self.InitActorLocation` (`self.K2_GetActorLocation`))
  (bind (_direction _alpha) (`Timeline|MoveToPlayer`)
    (:`Update`
      (`self.K2_SetActorLocation` (`KismetMathLibrary.VLerp` (`self.InitActorLocation`) (`self.K2_GetActorLocation` (`self.Player`)) _alpha)))
    (:`Finished`
      (`self.FinishCollect`))))

(event `FinishCollect`
  (`/Game/RPG_Game/Actors/Item/C_InventoryManager.Client_AddMoney` (`/Game/RPG_Game/Blueprints/RPG_PlayerController.C_InventoryManager` (cast `/Game/RPG_Game/Blueprints/RPG_PlayerController` (`Pawn.GetController` (`self.Player`)) :!pure true)) (`self.Money`))
  (`self.K2_DestroyActor`))

(fn `UserConstructionScript`)