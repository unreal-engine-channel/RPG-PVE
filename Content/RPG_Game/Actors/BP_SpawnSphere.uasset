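; BP_SpawnSphere is a spawner actor that respawns enemies at random reachable points within its sphere radius after a delay.
; RespawnEnemy queues an enemy class with its remaining time and starts a looping timer if none is running.
; Each timer tick counts down entries, spawns expired ones with itself as RespawnActor, and shifts pending indices as entries are removed.
; The timer clears itself once the queue is empty.
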(event `RespawnEnemy`
  (params (NewItem :type "/Game/RPG_Game/Blueprints/Structure/S_RespawnEnemy Structure (by ref)"))
  (`KismetArrayLibrary.Array_Add` (`self.EnemyList`) NewItem)
  (if (not (`KismetSystemLibrary.K2_IsValidTimerHandle` (`self.SpawnTimer`)))
    (bind _returnvalue (`KismetSystemLibrary.K2_SetTimerDelegate` (delegate `RespawnTick`) 0.5 true))
    (set `self.SpawnTimer` _returnvalue)))

(event `RespawnTick`
  (bind _indicestospawn (`self.IndicesToSpawn`))
  (for (_array_element _array_index) (`self.EnemyList`)
    (bind _returnvalue (- (break `/Game/RPG_Game/Blueprints/Structure/S_RespawnEnemy` _array_element) 0.5))
    (if (> _returnvalue 0.0)
      (`KismetArrayLibrary.Array_Set` (`self.EnemyList`) _array_index (make `/Game/RPG_Game/Blueprints/Structure/S_RespawnEnemy` _returnvalue (`.Enemy_6_480F7BCD414BC79E787436A71CCBE2D0` (break `/Game/RPG_Game/Blueprints/Structure/S_RespawnEnemy` _array_element))))
      (else
        (`KismetArrayLibrary.Array_Add` (`self.IndicesToSpawn`) _array_index))))
  (for _array_element_2 (`self.IndicesToSpawn`)
    (`|SpawnActorFromClass` (`.Enemy_6_480F7BCD414BC79E787436A71CCBE2D0` (break `/Game/RPG_Game/Blueprints/Structure/S_RespawnEnemy` (`|GetArrayItem` (`self.EnemyList`) _array_element_2))) (`KismetMathLibrary.MakeTransform` (`NavigationSystemV1.K2_GetRandomReachablePointInRadius` (`self.K2_GetActorLocation`) (`SphereComponent.SphereRadius` (`self.Sphere`)) null null)) "Undefined" "OverrideRootScale" null self null)
    (`KismetArrayLibrary.Array_Remove` (`self.EnemyList`) _array_element_2)
    (for _index (range _array_element_2 (+ (`KismetArrayLibrary.Array_LastIndex` (`self.IndicesToSpawn`)) 1))
      (`KismetArrayLibrary.Array_Set` _indicestospawn _index (- (`|GetArrayItem` _indicestospawn _index) 1))))
  (`KismetArrayLibrary.Array_Clear` (`self.IndicesToSpawn`))
  (if (not (> (`KismetArrayLibrary.Array_Length` (`self.EnemyList`)) 0))
    (`KismetSystemLibrary.K2_ClearAndInvalidateTimerHandle` (`self.SpawnTimer`))))

(fn `UserConstructionScript`)