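; Quest-giver NPC for the RPG that offers quests unlocked by the player's level.
; The player's level event drives UpdateQuest, which steps through the QuestInLevel map and switches the sprite to a question mark.
; A sphere overlap toggles the named interaction widget; interacting in range adds the quest to QuestManage unstarted and restores the circle sprite.
; The player is set as owner so the sprite is hidden from their view.
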(event `self.ReceiveBeginPlay`
  (bind _shibi (`self.Shibi`))
  (bind _asbp_player (cast `/Game/RPG_Game/Blueprints/BP_Player` (`GameplayStatics.GetPlayerCharacter` 0)))
  (set `self.Shibi` _asbp_player)
  (`self.SetOwner` _asbp_player)
  (`PrimitiveComponent.SetOwnerNoSee` (`self.PaperSprite`) true)
  (bind _asw_interaction (cast `/Game/RPG_Game/UI/W_Interaction` (`WidgetComponent.GetUserWidgetObject` (`self.Widget`))))
  (`TextBlock.SetText` (`/Game/RPG_Game/UI/W_Interaction.Name` _asw_interaction) (`self.Name`))
  (add `/Game/RPG_Game/Blueprints/BP_Player.OnInteract` _shibi (`|CreateDelegate` :!event `OnInteract`))
  (add `/Game/RPG_Game/Blueprints/BP_Player.UpdateLevelForQuest` _shibi (`|CreateDelegate` :!event `UpdateQuest`))
  (`self.UpdateQuest` 0))

(event `OnInteract`
  (if (and (`self.HasQuest?`) (`self.InRadius?`) (`KismetSystemLibrary.IsValidClass` (`self.CurrentQuestClass`)))
    (`/Game/RPG_Game/Component/QuestManager.AddQuest` (`/Game/RPG_Game/Blueprints/BP_RPG_Character.QuestManage` (`self.Shibi`)) (`self.CurrentQuestClass`) false)
    (set `self.HasQuest?` false)
    (`PaperSpriteComponent.SetSprite` (`self.PaperSprite`) "/Game/RPG_Game/Textures/circle_Sprite.circle_Sprite")))

(event `self.Sphere.OnComponentBeginOverlap`
  (params (OverlappedComponent :type "PrimitiveComponent Object Reference") (OtherActor :type "Actor Object Reference") (OtherComp :type "PrimitiveComponent Object Reference") (OtherBodyIndex :type Integer) (bFromSweep :type Boolean) (SweepResult :type "HitResult Structure (by ref)"))
  (if (== OtherActor (`self.Shibi`))
    (`SceneComponent.SetHiddenInGame` (`self.Widget`) false false)
    (set `self.InRadius?` true)))

(event `self.Sphere.OnComponentEndOverlap`
  (params (OverlappedComponent :type "PrimitiveComponent Object Reference") (OtherActor :type "Actor Object Reference") (OtherComp :type "PrimitiveComponent Object Reference") (OtherBodyIndex :type Integer))
  (if (== OtherActor (`self.Shibi`))
    (`SceneComponent.SetHiddenInGame` (`self.Widget`) true false)
    (set `self.InRadius?` false)))

(event `UpdateQuest`
  (params (Level :type Integer))
  (bind _questinlevel (`self.QuestInLevel`))
  (bind _keys (`BlueprintMapLibrary.Map_Keys` _questinlevel))
  (bind _output (`|GetArrayItem` _keys (`self.LevelIndex`)))
  (bind _value (`BlueprintMapLibrary.Map_Find` _questinlevel _output))
  (if (and (>= Level _output) (`KismetSystemLibrary.IsValidClass` _value) (!= (`self.CurrentQuestClass`) _value))
    (set `self.HasQuest?` true)
    (`PaperSpriteComponent.SetSprite` (`self.PaperSprite`) "/Game/RPG_Game/Textures/question_mark_Sprite.question_mark_Sprite")
    (set `self.CurrentQuestClass` _value)
    (`/Engine/EditorBlueprintResources/StandardMacros.IncrementInt` (`self.LevelIndex`))))

(fn `UserConstructionScript`
  (`parent.UserConstructionScript`))