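; Enemy character for an RPG, with level-scaled attributes and rewards, an attached weapon and an overlap-shown nameplate colored relative to player level.
; Sighting the player or taking damage sets the blackboard target and switches BehaviorComponent state.
; Damage runs through defense and critical calculation, driving hit montages, knockback, floating numbers and the health bar.
; Death waits out its montage, spawns XP and money pickups, requests a respawn and destroys the enemy.
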(event `self.ReceiveBeginPlay`
  (bind _asbp_player (cast `/Game/RPG_Game/Blueprints/BP_Player` (`GameplayStatics.GetPlayerCharacter` 0) :!pure true))
  (`parent.ReceiveBeginPlay`)
  (`self.UpdateAttribute`)
  (`self.CreateWeapon`)
  (`self.SetOwner` (`GameplayStatics.GetPlayerCharacter` 0))
  (`PrimitiveComponent.SetOwnerNoSee` (`self.PaperSprite`) true)
  (`SceneComponent.SetVisibility` (`self.PaperSprite`) true false)
  (`self.SetHealthPercent`)
  (set `CharacterMovementComponent.MaxWalkSpeed` 200.0 (`self.CharacterMovement`))
  (`BlackboardComponent.SetValueAsVector` (`AIBlueprintHelperLibrary.GetBlackboard` null) "Original" (`self.K2_GetActorLocation`))
  (`BlackboardComponent.SetValueAsFloat` (`AIBlueprintHelperLibrary.GetBlackboard` null) "RandomRange" (`self.RandomRange`))
  (`self.SetNameAndLevel` (`/Game/RPG_Game/Blueprints/BP_Player.Level` _asbp_player))
  (set `self.Player` _asbp_player)
  (add `/Game/RPG_Game/Blueprints/BP_Player.UpdateLevelForQuest` _asbp_player (`|CreateDelegate` :!event `UpdateLevelColor`))
  (`/Game/RPG_Game/Component/BehaviorComponent.SetBehavior` (`self.BehaviorComponent`) "NewEnumerator4"))

(event `self.PawnSensing.OnSeePawn`
  (params (Pawn :type "Pawn Object Reference"))
  (if (== Pawn (`GameplayStatics.GetPlayerPawn` 0))
    (`BlackboardComponent.SetValueAsObject` (`AIBlueprintHelperLibrary.GetBlackboard` null) "Target" Pawn)
    (set `CharacterMovementComponent.MaxWalkSpeed` 400.0 (`self.CharacterMovement`))
    (`/Engine/EditorBlueprintResources/StandardMacros.DoOnce` false :!label _label
      (:`Completed`
        (`/Game/RPG_Game/Component/BehaviorComponent.SetBehavior` (`self.BehaviorComponent`) "NewEnumerator5")))))

(event `Reset`
  (set `CharacterMovementComponent.MaxWalkSpeed` 200.0 (`self.CharacterMovement`))
  (`/Game/RPG_Game/Component/BehaviorComponent.SetBehavior` (`self.BehaviorComponent`) "NewEnumerator4")
  (goto _label :!via `Reset`))

(event `UpdateLevelColor`
  (params (Level :type Integer))
  (`self.SetNameAndLevel` Level))

(event `Attack`
  (params (NewParam :type "/Game/RPG_Game/AI/BTTask/BTTask_Attack Object Reference"))
  (bind _currentmontage (`self.CurrentMontage`))
  (`self.K2_SetActorRotation` (`KismetMathLibrary.FindLookAtRotation` (`self.K2_GetActorLocation`) (`self.K2_GetActorLocation` (`GameplayStatics.GetPlayerCharacter` 0))))
  (`/Engine/EditorBlueprintResources/StandardMacros.IsValid` _currentmontage
    (:`Is Valid`
      (bind _returnvalue (`self.PlayAnimMontage` _currentmontage))
      (`KismetSystemLibrary.Delay` _returnvalue)
      (`/Game/RPG_Game/AI/BTTask/BTTask_Attack.FinalAttack` NewParam))))

(event `CreateWeapon`
  (if (`KismetSystemLibrary.IsValidClass` (`self.Weapon`))
    (bind _returnvalue (`|SpawnActorFromClass` (`self.Weapon`) (`KismetMathLibrary.MakeTransform` (0.0 0.0 0.0)) "AlwaysSpawn" "OverrideRootScale" null self null))
    (bind _output_get (set `self.CurrentWeapon` _returnvalue))
    (`self.K2_AttachToComponent` _output_get (`self.Mesh`) "Weapon" "KeepRelative" "KeepRelative" "KeepRelative" true)))

(event `/Game/RPG_Game/Blueprints/Interface/I_Damageable.OnRecieveDamage`
  (params (PhysicalDamage :type "Float (single-precision)") (MagicDamage :type "Float (single-precision)") (CriticalChance :type "Float (single-precision)") (CriticalDamage :type "Float (single-precision)") (Attacker :type "Actor Object Reference"))
  (bind (_currenthealth _maxhealth _criticalchance _physicaldamage _magicdamage _physicaldefence _magicdefence) (break `/Game/RPG_Game/Blueprints/Structure/S_EnemyAttribute` (`self.Attribute`)))
  (if (`self.IsAlive?`)
    (set `self.CurrentAttacker` Attacker)
    (bind (_iscritical_ _damage) (`self.CalculateDamage` PhysicalDamage MagicDamage CriticalChance CriticalDamage _physicaldefence _magicdefence))
    (`|ExecutionSequence`
      (:`then_0`
        (if (not (`BlackboardComponent.GetValueAsBool` (`AIBlueprintHelperLibrary.GetBlackboard` null) "IsRunningBack?"))
          (`self.PlayAnimMontage` (select `bool` _iscritical_ :`false` (`self.ReactHit`) :`true` (`self.ReactHeavyHit`)) 1.0 (`KismetStringLibrary.Conv_StringToName` (`KismetStringLibrary.Conv_IntToString` (`KismetMathLibrary.RandomInteger` 2))))
          (if _iscritical_
            (`self.LaunchCharacter` (* (`self.GetActorForwardVector` (`GameplayStatics.GetPlayerCharacter` 0)) 200.0)))))
      (:`then_1`
        (`self.ModifyValue` _iscritical_ (* _damage -1.0))))))

(event `ModifyValue`
  (params (Critical :type Boolean) (Damage :type "Float (double-precision)"))
  (bind _attribute (`self.Attribute`))
  (bind _behaviorcomponent (`self.BehaviorComponent`))
  (bind (_currenthealth _maxhealth _criticalchance _physicaldamage _magicdamage _physicaldefence _magicdefence) (break `/Game/RPG_Game/Blueprints/Structure/S_EnemyAttribute` _attribute))
  (bind _returnvalue (`AddComponent|NODE_AddWC_OnDamaged-0` :`bManualAttachment` true :`RelativeTransform` (`self.GetTransform`)))
  (`/Game/RPG_Game/UI/WC_OnDamaged.SetDamageText` _returnvalue Damage (>= Damage 0.0) "NewEnumerator0" Critical false)
  (setmembers `/Game/RPG_Game/Blueprints/Structure/S_EnemyAttribute` :`StructRef` _attribute :`CurrentHealth` (+ _currenthealth Damage))
  (`self.SetHealthPercent`)
  (if (<= _currenthealth 0.0)
    (`/Game/RPG_Game/Component/BehaviorComponent.SetBehavior` _behaviorcomponent "NewEnumerator6")
    (else
      (`BlackboardComponent.SetValueAsObject` (`AIBlueprintHelperLibrary.GetBlackboard` null) "Target" (`self.CurrentAttacker`))
      (`/Game/RPG_Game/Component/BehaviorComponent.SetBehavior` _behaviorcomponent "NewEnumerator5"))))

(event `OnDeath`
  (bind _respawnactor (`self.RespawnActor`))
  (bind _currentweapon (`self.CurrentWeapon`))
  (`SceneComponent.SetVisibility` (`self.NameAndHealthBar`) false false)
  (`SceneComponent.SetVisibility` (`self.PaperSprite`) false false)
  (`self.DetachFromControllerPendingDestroy`)
  (`self.PlayAnimMontage` (`self.Deatth`) 1.0 (`KismetStringLibrary.Conv_StringToName` (`KismetStringLibrary.Conv_IntToString` (`KismetMathLibrary.RandomInteger` 7))))
  (if (not (`self.IsPlayingMontage`)) :!label _label_2
    (`self.SpawnXPAndMoney` (`KismetMathLibrary.RandomIntegerInRange` 1 3))
    (`/Engine/EditorBlueprintResources/StandardMacros.IsValid` _respawnactor
      (:`Is Valid`
        (`/Game/RPG_Game/Actors/BP_SpawnSphere.RespawnEnemy` _respawnactor (make `/Game/RPG_Game/Blueprints/Structure/S_RespawnEnemy` (`self.RespawnTime`) (`GameplayStatics.GetObjectClass` self))))
      (:`Is Not Valid`
        _))
    (`self.K2_DestroyActor`)
    (`/Engine/EditorBlueprintResources/StandardMacros.IsValid` _currentweapon
      (:`Is Valid`
        (`self.K2_DestroyActor` _currentweapon)))
    (else
      (`KismetSystemLibrary.Delay` 0.01)
      (goto _label_2))))

(event `self.ShowEnemyWidget.OnComponentBeginOverlap`
  (params (OverlappedComponent :type "PrimitiveComponent Object Reference") (OtherActor :type "Actor Object Reference") (OtherComp :type "PrimitiveComponent Object Reference") (OtherBodyIndex :type Integer) (bFromSweep :type Boolean) (SweepResult :type "HitResult Structure (by ref)"))
  (if (`PrimitiveComponent.IsOverlappingActor` (`self.ShowEnemyWidget`) (`GameplayStatics.GetPlayerCharacter` 0))
    (`SceneComponent.SetVisibility` (`self.NameAndHealthBar`) true false)))

(event `self.ShowEnemyWidget.OnComponentEndOverlap`
  (params (OverlappedComponent :type "PrimitiveComponent Object Reference") (OtherActor :type "Actor Object Reference") (OtherComp :type "PrimitiveComponent Object Reference") (OtherBodyIndex :type Integer))
  (if (not (`PrimitiveComponent.IsOverlappingActor` (`self.ShowEnemyWidget`) (`GameplayStatics.GetPlayerCharacter` 0)))
    (`SceneComponent.SetVisibility` (`self.NameAndHealthBar`) false false)))

(fn `IsAlive?`
  (returns (ReturnValue :type Boolean))
  (return (> (`.CurrentHealth_15_3F7F3B764EC5F254CBD11A827F1FAAC3` (break `/Game/RPG_Game/Blueprints/Structure/S_EnemyAttribute` (`self.Attribute`))) 0.0)))

(fn `IsPlayingMontage`
  (returns (Out :type Boolean))
  (bind _returnvalue (`self.GetCurrentMontage`))
  (return (`KismetSystemLibrary.IsValid` _returnvalue)))

(fn `SetHealthPercent`
  (bind (_currenthealth _maxhealth) (break `/Game/RPG_Game/Blueprints/Structure/S_EnemyAttribute` (`self.Attribute`)))
  (`ProgressBar.SetPercent` (`/Game/RPG_Game/UI/W_Enemy.Health` (cast `/Game/RPG_Game/UI/W_Enemy` (`WidgetComponent.GetUserWidgetObject` (`self.NameAndHealthBar`)) :!pure true)) (/ _currenthealth _maxhealth))
  (return))

(fn `SetNameAndLevel`
  (params (PlayerLevel :type Integer))
  (bind _returnvalue (`KismetMathLibrary.Conv_IntToDouble` PlayerLevel))
  (bind _level (`self.Level`))
  (bind _xp_points (`self.XP_Points`))
  (bind _returnvalue_2 (`KismetMathLibrary.Conv_IntToDouble` _level))
  (bind _returnvalue_3 (- (`self.Level`) PlayerLevel))
  (bind _name (`/Game/RPG_Game/UI/W_Enemy.Name` (cast `/Game/RPG_Game/UI/W_Enemy` (`WidgetComponent.GetUserWidgetObject` (`self.NameAndHealthBar`)) :!pure true)))
  (set `self.XP_Points` (select `bool` (> _returnvalue_3 0) :`false` _xp_points :`true` (+ _xp_points (`KismetMathLibrary.Conv_IntToDouble` _returnvalue_3))))
  (`TextBlock.SetText` _name (`|FormatText` "[Lvl {Level}] {Name}" _level (`self.Name`)))
  (`TextBlock.SetColorAndOpacity` _name (make `SlateColor` (select `bool` (>= _level (+ PlayerLevel 5)) :`false` (select `bool` (<= _level (- PlayerLevel 1)) :`false` (`KismetMathLibrary.LinearColorLerpUsingHSV` (struct :`R` 1.0 :`A` 1.0) (struct :`G` 1.0 :`A` 1.0) (/ (`KismetMathLibrary.SelectFloat` 1.0 _returnvalue (<= _returnvalue 0.0)) (`KismetMathLibrary.SelectFloat` 1.0 _returnvalue_2 (<= _returnvalue_2 0.0)))) :`true` (struct :`R` 1.0 :`G` 1.0 :`B` 1.0 :`A` 1.0)) :`true` (struct :`R` 1.0 :`B` 0.009159 :`A` 1.0)))))

(fn `SpawnXPAndMoney`
  (params (FirstIndex :type Integer))
  (bind _player (`self.Player`))
  (bind _returnvalue (`KismetMathLibrary.Conv_VectorToTransform` (`KismetMathLibrary.RandomPointInBoundingBox` (`self.K2_GetActorLocation`))))
  (for _ (range (+ FirstIndex 1))
    (`|SpawnActorFromClass` "/Game/RPG_Game/Actors/BP_XP.BP_XP_C" _returnvalue "Undefined" "OverrideRootScale" null _player (`self.XP_Points`) null)
    (`|SpawnActorFromClass` "/Game/RPG_Game/Actors/BP_SpawnMoney.BP_SpawnMoney_C" _returnvalue "Undefined" "OverrideRootScale" null _player (`self.Money`) null)))

(fn `UpdateAttribute`
  (bind _attribute (`self.Attribute`))
  (bind (_currenthealth _maxhealth _criticalchance _physicaldamage _magicdamage _physicaldefence _magicdefence) (break `/Game/RPG_Game/Blueprints/Structure/S_EnemyAttribute` _attribute))
  (bind _returnvalue (+ _maxhealth 50.0))
  (for _ (range 1 (+ (`self.Level`) 1))
    (setmembers `/Game/RPG_Game/Blueprints/Structure/S_EnemyAttribute` :`StructRef` _attribute :`CurrentHealth` _returnvalue :`MaxHealth` _returnvalue :`CriticalChance` (+ _criticalchance 1.0) :`PhysicalDamage` (+ _physicaldamage 15.0) :`MagicDamage` (+ _magicdamage 20.0) :`PhysicalDefence` (+ _physicaldefence 10.0) :`MagicDefence` (+ _magicdefence 10.0))
    (set `self.XP_Points` (+ (`self.XP_Points`) 2.0))
    (set `self.Money` (+ (`self.Money`) 2))))

(fn `UserConstructionScript`
  (`parent.UserConstructionScript`))