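; RPG character Blueprint whose only logic is a damage calculation function; its event graph and construction script are empty.
; CalculateDamage randomizes physical or magic damage, with wider variance for magic, subtracts the matching defence, then rolls for a critical multiplier and rounds.
; The physical branch returns first, so magic is evaluated only without positive physical damage.
; AbsoluteDefence skips the calculation entirely.
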(fn `CalculateDamage`
  (params (PhysicalDamage :type "Float (double-precision)") (MagicDamage :type "Float (double-precision)") (CriticalChance :type "Float (double-precision)") (CriticalDamage :type "Float (double-precision)") (PhysicalDefence :type "Float (double-precision)") (MagicDefence :type "Float (double-precision)") (AbsoluteDefence :type Boolean))
  (returns (`IsCritical?` :type Boolean) (Damage :type "Float (double-precision)"))
  (locals (LocalPhysicalDamage :type "Float (double-precision)" :default 0.0) (LocalMagicDamage :type "Float (double-precision)" :default 0.0) (LocalDamage :type "Float (double-precision)") (LocalCritical :type Boolean))
  (if (not AbsoluteDefence)
    (`|ExecutionSequence`
      (:`then_0`
        (if (> PhysicalDamage 0.0)
          (set `local.LocalPhysicalDamage` (- (* PhysicalDamage (`KismetMathLibrary.RandomFloatInRange` 0.9 1.1)) PhysicalDefence))
          (set `local.LocalDamage` (+ (`local.LocalPhysicalDamage`) (`local.LocalMagicDamage`)) :!label _label)
          (bind _output_get (set `local.LocalCritical` (<= (`KismetMathLibrary.RandomFloatInRange` 1.0 100.0) (`local.CriticalChance`))))
          (bind _output_get_2 (set `local.LocalDamage` (* (`local.LocalDamage`) (select `bool` (`local.LocalCritical`) :`false` 1.0 :`true` (`local.CriticalDamage`)))))
          (return _output_get (`KismetMathLibrary.Conv_IntToDouble` (`KismetMathLibrary.Round` _output_get_2)))))
      (:`then_1`
        (if (> MagicDamage 0.0)
          (set `local.LocalMagicDamage` (- (* MagicDamage (`KismetMathLibrary.RandomFloatInRange` 0.7 1.3)) MagicDefence))
          (goto _label))))))

(fn `UserConstructionScript`)