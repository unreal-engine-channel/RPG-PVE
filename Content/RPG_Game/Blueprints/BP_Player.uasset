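; RPG player character handling HUD, melee combat, double jump, interaction, quests, levelling and money.
; An attribute map drives Health, Mana and Stamina bars, with looping regen timers paused when full; recent attribute loss blocks Health and Mana regen.
; Stamina-gated three-hit combo buffers input for SaveAttack, while LineAttack traces forward to damage I_Damageable pawns.
; Money counts toward its target by timer; several keys are test hooks for attributes, XP and quests.
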(event `self.ReceiveBeginPlay`
  (set `/Game/RPG_Game/Component/QuestManager.Shibi` self (`self.QuestManage`))
  (bind _returnvalue (`|CreateWidget` "/Game/RPG_Game/UI/W_PC_Main.W_PC_Main_C" null self))
  (bind _output_get (set `self.MasterWidget` _returnvalue))
  (`self.SetupAttributeBars`)
  (`self.UpdateAttribute` "NewEnumerator0")
  (`self.UpdateAttribute` "NewEnumerator1")
  (`self.Regenerations`)
  (`UserWidget.AddToViewport` _output_get 0)
  (add `/Game/RPG_Game/UI/W_Level.UpdateLevel` (`/Game/RPG_Game/UI/W_PC_Main.W_Level` (`self.MasterWidget`)) (`|CreateDelegate` :!event `UpLevel`)))

(event `Key|Subtract`
  (params (Key :type "Key Structure"))
  (:`Pressed`
    (`self.GetMoney` -1000)
    (`self.ModifyAttribute` "NewEnumerator0" -30.0)
    (`KismetSystemLibrary.Delay` 0.2)
    (`self.ModifyAttribute` "NewEnumerator1" -30.0)
    (`KismetSystemLibrary.Delay` 0.2)
    (`self.ModifyAttribute` "NewEnumerator2" -30.0)))

(event `UpLevel`
  (params (Level :type Integer))
  (bind _charactermovement (`self.CharacterMovement`))
  ;[1 1 1] 角色升级
  (`self.UpdateLevelForQuest` Level)
  (bind _output_get (set `self.Level` Level))
  (set `/Game/RPG_Game/UI/W_CharacterBorder.LevelText` (`KismetTextLibrary.Conv_IntToText` _output_get) (`/Game/RPG_Game/UI/W_PC_Main.W_CharacterBorder` (`self.MasterWidget`)))
  (`self.UpdateLevel`)
  (set `CharacterMovementComponent.MaxWalkSpeed` 0.0 _charactermovement)
  (`self.PlayAnimMontage` "/Game/RPG_Game/Characters/Shibi/Animations/Montage/UpLevel_HappyClap_Montage.UpLevel_HappyClap_Montage" 1.5)
  (`KismetSystemLibrary.Delay` 2.0)
  (set `CharacterMovementComponent.MaxWalkSpeed` 600.0 _charactermovement))

(event `Key|Add`
  (params (Key :type "Key Structure"))
  (:`Pressed`
    (`self.GetMoney` 1000)
    (`self.ModifyAttribute` "NewEnumerator0" 30.0)
    (`KismetSystemLibrary.Delay` 0.2)
    (`self.ModifyAttribute` "NewEnumerator1" 30.0)
    (`KismetSystemLibrary.Delay` 0.2)
    (`self.ModifyAttribute` "NewEnumerator2" 30.0)))

(event `Key|F`
  (params (Key :type "Key Structure"))
  (:`Pressed`
    (`self.AddXP` 150.0)))

(event `AddXP`
  (params (XP :type "Float (double-precision)"))
  (`/Game/RPG_Game/UI/W_Level.GetXP` (`/Game/RPG_Game/UI/W_PC_Main.W_Level` (`self.MasterWidget`)) XP))

(event `Key|SpaceBar`
  (params (Key :type "Key Structure"))
  (:`Pressed`
    (if (`self.IsAttacking?`)
      _
      (elif (>= (`.CurrentValue_2_54F26D6C45503B625A635DB5DB0959B0` (break `/Game/RPG_Game/Blueprints/Structure/S_Attribute` (`self.GetAttribute` "NewEnumerator2"))) 10.0)
        (bind _counter (`/Engine/EditorBlueprintResources/StandardMacros.Do N` 2 :!label _label)
          (:`Exit`
            (switch `int` _counter
              (:`1`
                (`self.Jump`))
              (:`2`
                (`self.LaunchCharacter` (0.0 0.0 600.0) false true)))
            (`GameplayStatics.PlaySoundAtLocation` "/Game/RPG_Game/Audio/Shibi/Shinbi_Effort_Jump.Shinbi_Effort_Jump" (`self.K2_GetActorLocation`) (struct) 1.0 1.0 0.0 null null null)
            (`self.ModifyAttribute` "NewEnumerator2" -5.0)))))))

(event `CoolDownFighting`
  (set `self.ResetTimer` 5)
  (bind _returnvalue (`KismetSystemLibrary.K2_SetTimerDelegate` (delegate `CountTime`) 1.0 true)))

(event `self.OnLanded`
  (params (Hit :type "HitResult Structure (by ref)"))
  (goto _label :!via `Reset`))

(event `CountTime`
  (bind _result (`/Engine/EditorBlueprintResources/StandardMacros.DecrementInt` (`self.ResetTimer`))
    (:`  `
      (if (== _result 0)
        (set `self.IsFighting?` false)
        (`KismetSystemLibrary.K2_ClearAndInvalidateTimerHandle` (stale `CoolDownFighting` _returnvalue))))))

(event `Regenerations`
  (bind _keys (`BlueprintMapLibrary.Map_Keys` (`self.Attributes`)))
  (for _array_element _keys
    (bind _value (`self.GetAttribute` _array_element))
    (bind ((`RegenInterval_32_078A245B43611ECB75D615BD8BCCD030` _regeninterval) (`RegenFunctionName_34_D2E71D77441E1DAA0FF670BC839322EA` _regenfunctionname)) (break `/Game/RPG_Game/Blueprints/Structure/S_Attribute` _value))
    (bind _returnvalue (`KismetSystemLibrary.K2_SetTimer` null _regenfunctionname _regeninterval true))
    (bind _structout (setmembers `/Game/RPG_Game/Blueprints/Structure/S_Attribute` :`StructRef` _value :`RegenTimerHandle` _returnvalue))
    (`self.SetAttribute` _structout _array_element)
    (`self.HandleRegeneration` _array_element)))

(event `Key|G`
  (params (Key :type "Key Structure"))
  (:`Pressed`
    (`/Game/RPG_Game/Component/QuestManager.AddQuest` (`self.QuestManage`) "/Game/RPG_Game/Actors/Quest/BP_FirstQuestTest.BP_FirstQuestTest_C")))

(event `Key|J`
  (params (Key :type "Key Structure"))
  (bind _currentsubgoalindex (`self.CurrentSubGoalIndex`))
  (:`Pressed`
    (`/Game/RPG_Game/Actors/Quest/BP_MasterQuest.CompleteSubGoal` (`/Game/RPG_Game/Component/QuestManager.CurrentQuest` (`self.QuestManage`)) _currentsubgoalindex)
    (`/Engine/EditorBlueprintResources/StandardMacros.IncrementInt` _currentsubgoalindex)))

(event `self.Box.OnComponentBeginOverlap`
  (params (OverlappedComponent :type "PrimitiveComponent Object Reference") (OtherActor :type "Actor Object Reference") (OtherComp :type "PrimitiveComponent Object Reference") (OtherBodyIndex :type Integer) (bFromSweep :type Boolean) (SweepResult :type "HitResult Structure (by ref)"))
  (if (`KismetSystemLibrary.DoesImplementInterface` OtherActor "/Game/RPG_Game/Blueprints/Interface/I_Interaction.I_Interaction_C")
    (message `/Game/RPG_Game/Blueprints/Interface/I_Interaction.BeginOverlapTargetObject` OtherActor)))

(event `Key|E`
  (params (Key :type "Key Structure"))
  (:`Pressed`
    (`self.OnInteract`)
    (for _array_element (`PrimitiveComponent.GetOverlappingActors` (`self.Box`) null)
      (if (`KismetSystemLibrary.DoesImplementInterface` _array_element "/Game/RPG_Game/Blueprints/Interface/I_Interaction.I_Interaction_C")
        (message `/Game/RPG_Game/Blueprints/Interface/I_Interaction.OnInteractWith` _array_element self)
        (break)))))

(event `self.Box.OnComponentEndOverlap`
  (params (OverlappedComponent :type "PrimitiveComponent Object Reference") (OtherActor :type "Actor Object Reference") (OtherComp :type "PrimitiveComponent Object Reference") (OtherBodyIndex :type Integer))
  (if (`KismetSystemLibrary.DoesImplementInterface` OtherActor "/Game/RPG_Game/Blueprints/Interface/I_Interaction.I_Interaction_C")
    (message `/Game/RPG_Game/Blueprints/Interface/I_Interaction.EndOverlapTargetObject` OtherActor)))

(event `GetMoney`
  (params (Add :type Integer))
  (bind _handlemoneytime (`self.HandleMoneyTime`))
  (bind _output_get (set `self.MaxMoney` (+ (`self.MaxMoney`) Add)))
  (`/Engine/EditorBlueprintResources/StandardMacros.CompareInt` _output_get (`self.CurrentMoney`)
    (:`>`
      (set `self.IsAdd?` true)
      (if (`KismetSystemLibrary.K2_IsValidTimerHandle` _handlemoneytime) :!label _label_2
        (`KismetSystemLibrary.K2_UnPauseTimerHandle` _handlemoneytime)
        (else
          (bind _returnvalue (`KismetSystemLibrary.K2_SetTimer` null "CountMoney" 0.001 true))
          (set `self.HandleMoneyTime` _returnvalue))))
    (:`==`
      (`KismetSystemLibrary.K2_PauseTimerHandle` _handlemoneytime))
    (:`<`
      (set `self.IsAdd?` false)
      (goto _label_2))))

(event `MeleeAttack`
  ;[0.7708 0.1011 0.1073] 普通三连攻击
  (if (>= (`.CurrentValue_2_54F26D6C45503B625A635DB5DB0959B0` (break `/Game/RPG_Game/Blueprints/Structure/S_Attribute` (`self.GetAttribute` "NewEnumerator2"))) 15.0)
    (if (`self.IsAttacking?`)
      (set `self.CanGoToNextAttack?` true)
      (else
        (set `self.IsAttacking?` true)
        (switch `int` (`self.AttackCount`) :!label _label_3
          (:`0`
            (set `self.AttackCount` 1)
            (`self.PlayAnimMontage` "/Game/RPG_Game/Characters/Shibi/Animations/Montage/Melee_B.Melee_B")
            (`self.ModifyAttribute` "NewEnumerator2" -15.0))
          (:`1`
            (set `self.AttackCount` 2)
            (`self.PlayAnimMontage` "/Game/RPG_Game/Characters/Shibi/Animations/Montage/Melee_C.Melee_C")
            (`self.ModifyAttribute` "NewEnumerator2" -15.0))
          (:`2`
            (set `self.AttackCount` 0)
            (`self.PlayAnimMontage` "/Game/RPG_Game/Characters/Shibi/Animations/Montage/Melee_D.Melee_D")
            (`self.ModifyAttribute` "NewEnumerator2" -15.0)))))))

(event `SaveAttack`
  ;[0.7708 0.1011 0.1073] 普通三连攻击
  (if (`self.CanGoToNextAttack?`)
    (set `self.CanGoToNextAttack?` false)
    (goto _label_3)))

(event `ResetComb`
  ;[0.7708 0.1011 0.1073] 普通三连攻击
  (set `self.AttackCount` 0)
  (set `self.IsAttacking?` false)
  (set `self.CanGoToNextAttack?` false))

(event `/Game/RPG_Game/Blueprints/Interface/I_Damageable.OnRecieveDamage`
  (params (PhysicalDamage :type "Float (single-precision)") (MagicDamage :type "Float (single-precision)") (CriticalChance :type "Float (single-precision)") (CriticalDamage :type "Float (single-precision)") (Attacker :type "Actor Object Reference"))
  (`|ExecutionSequence`
    (:`then_0`
      (bind _returnvalue (`self.PlayAnimMontage` "/Game/RPG_Game/Characters/Shibi/Animations/HitReact_Back_Montage.HitReact_Back_Montage" 1.0 (`KismetStringLibrary.Conv_StringToName` (`KismetStringLibrary.Conv_IntToString` (`KismetMathLibrary.RandomIntegerInRange` 0 3)))))
      (`KismetSystemLibrary.Delay` _returnvalue)
      (`self.ResetComb`))
    (:`then_1`
      (bind (_iscritical_ _damage) (`self.CalculateDamage` PhysicalDamage MagicDamage CriticalChance 2.0 (`self.PhysicalDefence`) (`self.MagicDefence`) (`self.AbsoluteDefence`)))
      (`self.ModifyAttribute` "NewEnumerator0" (* _damage -1.0) _iscritical_))))

(event `Key|Q`
  (params (Key :type "Key Structure"))
  (:`Pressed`
    (if (`NavMovementComponent.IsFalling` (`self.CharacterMovement`))
      (`/Engine/EditorBlueprintResources/StandardMacros.DoOnce` false :!label _label_4
        (:`Completed`
          (bind _returnvalue (`self.PlayAnimMontage` "/Game/RPG_Game/Characters/Shibi/Animations/Montage/Air_Melee.Air_Melee"))
          (`KismetSystemLibrary.Delay` _returnvalue)
          (goto _label_4 :!via `Reset`)))
      (else
        (`self.MeleeAttack`)))))

(event `LineAttack`
  (bind _returnvalue (`self.K2_GetActorLocation`))
  (bind (_outhit _returnvalue_2) (`KismetSystemLibrary.LineTraceSingleForObjects` _returnvalue (+ _returnvalue (* (`self.GetActorForwardVector`) (`self.AttackRange`))) (`|MakeArray` "ObjectTypeQuery3" :!type "EObjectTypeQuery Enum")))
  (if _returnvalue_2
    (bind (_bblockinghit _binitialoverlap _time _distance _location _impactpoint _normal _impactnormal _physmat _hitactor) (`GameplayStatics.BreakHitResult` _outhit))
    (if (`KismetSystemLibrary.DoesImplementInterface` _hitactor "/Game/RPG_Game/Blueprints/Interface/I_Damageable.I_Damageable_C")
      (message `/Game/RPG_Game/Blueprints/Interface/I_Damageable.OnRecieveDamage` _hitactor (`self.PhysicalDamage`) (`self.MagicDamage`) (`self.CriticalChance`) (`self.CriticalDamage`) self))))

(fn `CountMoney`
  (bind _w_characterborder (`/Game/RPG_Game/UI/W_PC_Main.W_CharacterBorder` (`self.MasterWidget`)))
  (bind _output_get (set `self.CurrentMoney` (+ (`self.CurrentMoney`) (select `bool` (`self.IsAdd?`) :`false` -1 :`true` 1))))
  (`TextBlock.SetColorAndOpacity` (`/Game/RPG_Game/UI/W_CharacterBorder.MoenyText` _w_characterborder) (make `SlateColor` (select `bool` (> _output_get 0) :`false` (struct :`R` 1.0 :`B` 0.009159 :`A` 1.0) :`true` (struct :`R` 0.858333 :`G` 0.69585 :`B` 0.00058 :`A` 1.0) :!type "LinearColor Structure")))
  (set `/Game/RPG_Game/UI/W_CharacterBorder.Money` (`KismetTextLibrary.Conv_IntToText` (`self.CurrentMoney`)) _w_characterborder)
  (if (== (`self.MaxMoney`) (`self.CurrentMoney`))
    (`KismetSystemLibrary.K2_PauseTimerHandle` (`self.HandleMoneyTime`))))

(fn `GetAttribute`
  (params (Attribute :type "/Game/RPG_Game/Blueprints/Enum/E_Attribute Enum" :default "NewEnumerator3"))
  (returns (Value :type "/Game/RPG_Game/Blueprints/Structure/S_Attribute Structure"))
  (return (`BlueprintMapLibrary.Map_Find` (`self.Attributes`) Attribute)))

(fn `HandleRegeneration`
  (params (NewParam :type "/Game/RPG_Game/Blueprints/Enum/E_Attribute Enum" :default "NewEnumerator3"))
  (bind ((`CurrentValue_2_54F26D6C45503B625A635DB5DB0959B0` _currentvalue) (`MaxValue_8_66D7E0094450B66A1E1F60BC1632356D` _maxvalue) (`RegenTimerHandle_36_5AF0176F4043199E12B2AE9D16D014D1` _regentimerhandle)) (break `/Game/RPG_Game/Blueprints/Structure/S_Attribute` (`self.GetAttribute` NewParam)))
  (bind _returnvalue (`KismetSystemLibrary.K2_IsTimerPausedHandle` _regentimerhandle))
  (if (and (!= _currentvalue _maxvalue) _returnvalue)
    (`KismetSystemLibrary.K2_UnPauseTimerHandle` _regentimerhandle)
    (elif (and (== _currentvalue _maxvalue) (not _returnvalue))
      (`KismetSystemLibrary.K2_PauseTimerHandle` _regentimerhandle))))

(fn `HealthRegenTick`
  (bind ((`MaxValue_8_66D7E0094450B66A1E1F60BC1632356D` _maxvalue) (`RegenInterval_32_078A245B43611ECB75D615BD8BCCD030` _regeninterval) (`MaxRegenTime_33_D7AB0EC74AFEE8EE1378FCA2DCF2AF93` _maxregentime)) (break `/Game/RPG_Game/Blueprints/Structure/S_Attribute` (`self.GetAttribute` "NewEnumerator0")))
  (if (not (`self.IsFighting?`))
    (`self.ModifyAttribute` "NewEnumerator0" (* _maxvalue (/ _regeninterval _maxregentime)))))

(fn `ManaRegenTick`
  (bind ((`MaxValue_8_66D7E0094450B66A1E1F60BC1632356D` _maxvalue) (`RegenInterval_32_078A245B43611ECB75D615BD8BCCD030` _regeninterval) (`MaxRegenTime_33_D7AB0EC74AFEE8EE1378FCA2DCF2AF93` _maxregentime)) (break `/Game/RPG_Game/Blueprints/Structure/S_Attribute` (`self.GetAttribute` "NewEnumerator1")))
  (if (not (`self.IsFighting?`))
    (`self.ModifyAttribute` "NewEnumerator1" (* _maxvalue (/ _regeninterval _maxregentime)))))

(fn `ModifyAttribute`
  (params (Attribute :type "/Game/RPG_Game/Blueprints/Enum/E_Attribute Enum" :default "NewEnumerator3") (ModifyValue :type "Float (double-precision)") (Critical :type Boolean))
  (locals (LocalAttribute :type "/Game/RPG_Game/Blueprints/Enum/E_Attribute Enum" :default "NewEnumerator3") (LocalModifyValue :type "Float (double-precision)") (LocalMaxValue :type "Float (double-precision)"))
  (bind _localattribute (`local.LocalAttribute`))
  (bind _value (`self.GetAttribute` (`local.LocalAttribute`)))
  (bind ((`CurrentValue_2_54F26D6C45503B625A635DB5DB0959B0` _currentvalue) (`MaxValue_8_66D7E0094450B66A1E1F60BC1632356D` _maxvalue)) (break `/Game/RPG_Game/Blueprints/Structure/S_Attribute` (`self.GetAttribute` (`local.LocalAttribute`))))
  (bind (_currentvalue_2 _minvalue _maxvalue_2) (break `/Game/RPG_Game/Blueprints/Structure/S_Attribute` _value))
  (if (<= ModifyValue 0.0)
    (set `self.IsFighting?` true)
    (`self.CoolDownFighting`))
  (bind _returnvalue (`AddComponent|NODE_AddWC_OnDamaged-1` :`bManualAttachment` true :`RelativeTransform` (`self.GetTransform`)))
  (`/Game/RPG_Game/UI/WC_OnDamaged.SetDamageText` _returnvalue ModifyValue (>= ModifyValue 0.0) Attribute Critical true)
  (set `local.LocalAttribute` Attribute)
  (set `local.LocalModifyValue` (`KismetMathLibrary.Conv_IntToDouble` (`KismetMathLibrary.FTrunc` (`KismetMathLibrary.FClamp` ModifyValue (* _currentvalue -1.0) (- _maxvalue _currentvalue)))))
  (bind _structout (setmembers `/Game/RPG_Game/Blueprints/Structure/S_Attribute` :`StructRef` _value :`CurrentValue` (`KismetMathLibrary.FClamp` (+ _currentvalue_2 (`local.LocalModifyValue`)) _minvalue _maxvalue_2)))
  (`self.SetAttribute` _structout _localattribute)
  (`self.UpdateAttribute` _localattribute)
  (`self.HandleRegeneration` _localattribute))

(fn `SetAttribute`
  (params (Value :type "/Game/RPG_Game/Blueprints/Structure/S_Attribute Structure (by ref)") (Attribute :type "/Game/RPG_Game/Blueprints/Enum/E_Attribute Enum" :default "NewEnumerator3"))
  (`BlueprintMapLibrary.Map_Add` (`self.Attributes`) Attribute Value)
  (return))

(fn `SetupAttributeBars`
  (bind _masterwidget (`self.MasterWidget`))
  (bind _w_characterborder (`/Game/RPG_Game/UI/W_PC_Main.W_CharacterBorder` _masterwidget))
  (bind _structout (setmembers `/Game/RPG_Game/Blueprints/Structure/S_Attribute` :`StructRef` (`self.GetAttribute` "NewEnumerator0") :`GlassBallWidget` (`/Game/RPG_Game/UI/W_PC_Main.Health` _masterwidget) :`HealthBar` (`/Game/RPG_Game/UI/W_CharacterBorder.W_HealthBar` _w_characterborder)))
  (`self.SetAttribute` _structout "NewEnumerator0")
  (bind _structout_2 (setmembers `/Game/RPG_Game/Blueprints/Structure/S_Attribute` :`StructRef` (`self.GetAttribute` "NewEnumerator1") :`GlassBallWidget` (`/Game/RPG_Game/UI/W_PC_Main.Mana` _masterwidget) :`ManaBar` (`/Game/RPG_Game/UI/W_CharacterBorder.W_ManaBar` _w_characterborder)))
  (`self.SetAttribute` _structout_2 "NewEnumerator1")
  (bind _structout_3 (setmembers `/Game/RPG_Game/Blueprints/Structure/S_Attribute` :`StructRef` (`self.GetAttribute` "NewEnumerator2") :`Stamina` (`/Game/RPG_Game/UI/W_CharacterBorder.Stamina` _w_characterborder)))
  (`self.SetAttribute` _structout_3 "NewEnumerator2"))

(fn `StaminaRegenTick`
  (bind ((`MaxValue_8_66D7E0094450B66A1E1F60BC1632356D` _maxvalue) (`RegenInterval_32_078A245B43611ECB75D615BD8BCCD030` _regeninterval) (`MaxRegenTime_33_D7AB0EC74AFEE8EE1378FCA2DCF2AF93` _maxregentime)) (break `/Game/RPG_Game/Blueprints/Structure/S_Attribute` (`self.GetAttribute` "NewEnumerator2")))
  (`self.ModifyAttribute` "NewEnumerator2" (* _maxvalue (/ _regeninterval _maxregentime))))

(fn `UpdateAttribute`
  (params (Attribute :type "/Game/RPG_Game/Blueprints/Enum/E_Attribute Enum" :default "NewEnumerator3"))
  (bind (_currentvalue _minvalue _maxvalue _glassballwidget _healthbar _manabar _stamina) (break `/Game/RPG_Game/Blueprints/Structure/S_Attribute` (`self.GetAttribute` Attribute)))
  (bind _glassball (`/Game/RPG_Game/UI/W_GlassBall.GlassBall` _glassballwidget))
  (bind _returnvalue (`KismetMathLibrary.FClamp` (/ _currentvalue _maxvalue)))
  (bind _result (`|FormatText` "{Current}/{Max}" (`KismetMathLibrary.Round` _currentvalue) (`KismetMathLibrary.Round` _maxvalue)))
  (switch `/Game/RPG_Game/Blueprints/Enum/E_Attribute` Attribute
    (:`NewEnumerator0`
      (`TextBlock.SetText` (`/Game/RPG_Game/UI/W_HealthBar.HealthText` _healthbar) _result)
      (`ProgressBar.SetPercent` (`/Game/RPG_Game/UI/W_HealthBar.HealthBar` _healthbar) _returnvalue)
      (bind _returnvalue_2 (`Image.GetDynamicMaterial` _glassball))
      (`MaterialInstanceDynamic.SetScalarParameterValue` _returnvalue_2 "Percentage" _returnvalue)
      (`MaterialInstanceDynamic.SetVectorParameterValue` _returnvalue_2 "Color" (`KismetMathLibrary.LinearColorLerpUsingHSV` (struct :`R` 1.0 :`A` 1.0) (`/Game/RPG_Game/UI/W_GlassBall.Color` _glassballwidget) _returnvalue)))
    (:`NewEnumerator1`
      (`TextBlock.SetText` (`/Game/RPG_Game/UI/W_ManaBar.ManaText` _manabar) _result)
      (`ProgressBar.SetPercent` (`/Game/RPG_Game/UI/W_ManaBar.ManaBar` _manabar) _returnvalue)
      (bind _returnvalue_3 (`Image.GetDynamicMaterial` _glassball))
      (`MaterialInstanceDynamic.SetScalarParameterValue` _returnvalue_3 "Percentage" _returnvalue))
    (:`NewEnumerator2`
      (`ProgressBar.SetPercent` _stamina _returnvalue))))

(fn `UpdateLevel`
  (bind _value (`self.GetAttribute` "NewEnumerator2"))
  (bind _value_2 (`self.GetAttribute` "NewEnumerator0"))
  (bind _value_3 (`self.GetAttribute` "NewEnumerator1"))
  (setmembers `/Game/RPG_Game/Blueprints/Structure/S_Attribute` :`StructRef` _value_2 :`MaxValue` (+ (`.MinValue_4_94B772924492A543992D70AE335F18B1` (break `/Game/RPG_Game/Blueprints/Structure/S_Attribute` _value_2)) 100.0))
  (setmembers `/Game/RPG_Game/Blueprints/Structure/S_Attribute` :`StructRef` _value_3 :`MaxValue` (+ (`.MinValue_4_94B772924492A543992D70AE335F18B1` (break `/Game/RPG_Game/Blueprints/Structure/S_Attribute` _value_3)) 50.0))
  (setmembers `/Game/RPG_Game/Blueprints/Structure/S_Attribute` :`StructRef` _value :`MaxValue` (+ (`.MinValue_4_94B772924492A543992D70AE335F18B1` (break `/Game/RPG_Game/Blueprints/Structure/S_Attribute` _value)) 10.0))
  (set `self.PhysicalDamage` (+ (`self.PhysicalDamage`) 10.0))
  (set `self.MagicDamage` (+ (`self.MagicDamage`) 15.0))
  (set `self.PhysicalDefence` (+ (`self.PhysicalDefence`) 10.0))
  (set `self.MagicDefence` (+ (`self.MagicDefence`) 10.0))
  (set `self.AbilityPoints` (+ (`self.AbilityPoints`) 1)))

(fn `UserConstructionScript`
  (`parent.UserConstructionScript`))